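; BP_Arrow is a short-lived arrow actor that detects hits on caretakers and destroys itself three seconds after BeginPlay.
; Its Box overlap casts the other actor to BP_Caretaker, stores it, and copies it to the Toddler reference's CurrentHitCaretaker.
; A hit only records the caretaker and prints a debug message, with no damage or early destruction in this graph.
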(event OnComponentBeginOverlap(Box)
  (params (OverlappedComponent :type Primitive%20Component%20Object%20Reference) (OtherActor :type Actor%20Object%20Reference) (OtherComp :type Primitive%20Component%20Object%20Reference) (OtherBodyIndex :type Integer) (bFromSweep :type Boolean) (SweepResult :type Hit%20Result%20Structure%20%28by%20ref%29))
  (bind _asbp_caretaker (Utilities|Casting|CastToBP_Caretaker OtherActor))
  (bind _output_get (Variables|Default|SetHit%20caretaker _asbp_caretaker))
  (Variables|/Game/ThirdPerson/Blueprints/BP_Toddler.BP_Toddler_C|SetcurrentHitCaretaker (Variables|Default|GetToddler) _output_get)
  (Development|PrintString "Caretaker DOWN"))

(event EventBeginPlay
  (Utilities|FlowControl|Delay 3.0)
  (Actor|DestroyActor))

(event Collision|EventActorBeginOverlap
  (params (OtherActor :type Actor%20Object%20Reference)))

(event EventTick
  (params (DeltaSeconds :type Float%20%28single-precision%29)))

(fn ConstructionScript)